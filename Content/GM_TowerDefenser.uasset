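; GM_TowerDefenser is the tower defense game mode, holding the player's health (Vida) and money (Parne).
; On BeginPlay it creates the BP_HUD widget, and its damage, add-money and remove-money functions push updated values to that HUD.
; Starting waves calls the Spawner and hides the start button, which reappears when waves end.
; The zero-health check in HacerDano has no action yet.
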(event EventBeginPlay
  ;[0.15 0.15 0.15 0.5] Inicio de partida
  (bind _returnvalue (UserInterface|CreateWidget "/Game/HUD/BP_HUD.BP_HUD_C"))
  (bind _output_get (Variables|Default|SetHUD _returnvalue))
  (UserInterface|Viewport|AddtoViewport _output_get 0)
  (CallFunction|ActualizarVida)
  (CallFunction|ActualizarParne)
  (Variables|Default|SetBTN%20Empezar (Variables|/Game/HUD/BP_HUD.BP_HUD_C|GetBTN_Empezar (Variables|Default|GetHUD))))

(fn ConstructionScript)

(fn HacerDano
  (params (Dano :type Integer))
  (bind _output_get (Variables|Default|SetVida (- (Variables|Default|GetVida) Dano)))
  (CallFunction|ActualizarVida)
  (if (<= _output_get 0)
    _))

(fn AnadirParne
  (params (Dinero :type Integer))
  (Variables|Default|SetParne (+ (Variables|Default|GetParne) Dinero))
  (CallFunction|ActualizarParne))

(fn QuitarParne
  (params (Dinero :type Integer))
  (Variables|Default|SetParne (- (Variables|Default|GetParne) Dinero))
  (CallFunction|ActualizarParne))

(fn ActualizarVida
  (Default|ActualizarVida (Variables|Default|GetHUD) (Utilities|String|ToString(Integer) (Variables|Default|GetVida))))

(fn ActualizarParne
  (Default|ActualizarParne (Variables|Default|GetHUD) (Utilities|String|ToString(Integer) (Variables|Default|GetParne))))

(fn EmpezarOleadas
  (Default|EmpezarOleada (Variables|Default|GetSpawner))
  (Variables|/Script/UMG.Widget|SetVisibility (Variables|Default|GetBTN%20Empezar) "Hidden"))

(fn TerminarOleadas
  (Variables|/Script/UMG.Widget|SetVisibility (Variables|Default|GetBTN%20Empezar) "Visible"))