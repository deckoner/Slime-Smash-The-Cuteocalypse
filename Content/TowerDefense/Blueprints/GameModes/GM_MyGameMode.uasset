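; Tower defense game mode that tracks player money and health, starts rounds through the enemy spawner and pauses on defeat.
; Turret placement uses a looping timer and mouse traces to position a frame and hologram preview, turned red when a box trace finds a blocker.
; Building spawns the turret and deducts its class-default cost.
; Clicked towers are selected by trace for paid damage upgrades, with WBP_HUD reflecting state.
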(event Custom|GainMoney
  (params (EnemyValue :type Float%20%28double-precision%29))
  (bind _myhud (Variables|Default|GetMyHUD))
  ;[0.15 0.15 0.15 0.5] Gain money
  (bind _output_get (Variables|Default|SetPlayerMoney (+ (Variables|Default|GetPlayerMoney) EnemyValue)))
  (Default|SetMoneyText _myhud _output_get)
  (Default|PhaseBuild _myhud)
  (Default|ActiveonOffUpgradeDamage _myhud))

(event Custom|LoseHP
  (params (Enemydamage :type Float%20%28double-precision%29))
  ;[0.15 0.15 0.15 0.5] Lose hp
  (bind _output_get (Variables|Default|SetPlayerHealth (- (Variables|Default|GetPlayerHealth) Enemydamage)))
  (Default|SetHealthText (Variables|Default|GetMyHUD) _output_get)
  (if (<= (Variables|Default|GetPlayerHealth) 0.0)
    (CallFunction|Defeat)))

(event Custom|StartRound
  ;[0.15 0.15 0.15 0.5] Comment
  (bind _returnvalue (Actor|GetActorOfClass "/Game/TowerDefense/Blueprints/Core/BP_EnemySpawner.BP_EnemySpawner_C"))
  (Default|EnemySpawnCaller _returnvalue)
  (Variables|Default|SetWave%20Couter (Variables|/Game/TowerDefense/Blueprints/Core/BP_EnemySpawner.BP_EnemySpawner_C|GetWaveCouter _returnvalue)))

(event EventBeginPlay
  ;[0.15 0.15 0.15 0.5] Add text to hud
  (bind _returnvalue (UserInterface|CreateWidget "/Game/TowerDefense/Blueprints/Widgets/WBP_HUD.WBP_HUD_C"))
  (bind _output_get (Variables|Default|SetMyHUD _returnvalue))
  (Default|SetHealthText _output_get (Variables|Default|GetPlayerHealth))
  (Default|SetMoneyText _output_get (Variables|Default|GetPlayerMoney))
  (Default|SetCurrentWave _output_get (Variables|Default|GetWave%20Couter))
  (Utilities|FlowControl|DelayUntilNextTick)
  (UserInterface|Viewport|AddtoViewport _output_get 0)
  (Variables|Default|SetPlayerController (Game|GetPlayerController 0)))

(fn ConstructionScript)

(fn Defeat
  (bind _returnvalue (UserInterface|CreateWidget "/Game/TowerDefense/Blueprints/Widgets/WBP_GameOver.WBP_GameOver_C"))
  (UserInterface|Viewport|AddtoViewport _returnvalue 0)
  (Game|SetGamePaused true))

(fn NewTurretMode
  (params (TypeTurret1 :type BP%20Base%20Tower%20Class%20Reference) (NewTurretPreview1 :type BP%20Base%20Tower%20Preview%20Class%20Reference))
  (Variables|Default|SetTurretPreviewClass NewTurretPreview1)
  (Variables|Default|SetTypeTurretClass TypeTurret1)
  (bind _returnvalue (Utilities|Time|SetTimerbyEvent (EventDispatchers|CreateEvent :!event UpdateTurretPosition) 0.01 true))
  (Variables|Default|SetTimerTurretPosition _returnvalue))

(fn BuildTurret
  (if (Variables|Default|GetBuildIsValid)
    (Game|SpawnActorfromClass (Variables|Default|GetTypeTurretClass) (Math|Transform|MakeTransform (Transformation|GetActorLocation (Variables|Default|GetTurretPreview)) "0, 0, 0" "1.000000,1.000000,1.000000") "Undefined" "MultiplyWithRoot" 0 0)
    (CallFunction|PayTurret (.Cost (Utilities|GetClassDefaults (Variables|Default|GetTypeTurretClass))))
    (CallFunction|CleanBuildVariable)))

(fn UpdateTurretPosition
  (bind _playercontroller (Variables|Default|GetPlayerController))
  (bind (_worldlocation _worlddirection) (Game|Player|ConvertMouseLocationToWorldSpace _playercontroller))
  (if (Variables|Default|GetBuildMode)
    (Class|WidgetLayoutLibrary|GetMousePositiononPlatform)
    (bind (_outhit _returnvalue) (Collision|LineTraceByChannel _worldlocation (+ _worldlocation (* _worlddirection 10000)) "TraceTypeQuery1" false 0 "None" true "(R=1.000000,G=0.000000,B=0.000000,A=0.000000)" "(R=1.000000,G=1.000000,B=1.000000,A=0.000000)"))
    (if _returnvalue
      (bind _output_get (LocalVariables|SetTurretPosistion (Math|Vector|MakeVector (.x (Transformation|GetActorLocation (.HitActor (Collision|BreakHitResult _outhit)))) (.y (Transformation|GetActorLocation (.HitActor (Collision|BreakHitResult _outhit)))) 4e+01)))
      (bind _frame (Variables|Default|GetFrame)
        (:then
          (Transformation|SetActorLocation _frame (LocalVariables|GetTurretPosistion) false true))
        (:else
          (bind _returnvalue_2 (Game|SpawnActorfromClass "/Game/TowerDefense/Blueprints/Towers/BP_FrameTower.BP_FrameTower_C" (Math|Transform|MakeTransform _output_get "0, 0, 0" "1.000000,1.000000,1.000000") "AlwaysSpawn" "MultiplyWithRoot" 0 0))
          (Variables|Default|SetFrame _returnvalue_2)))
      (bind _turretpreview (Variables|Default|GetTurretPreview)
        (:then
          (Transformation|SetActorLocation _turretpreview (LocalVariables|GetTurretPosistion) false true))
        (:else
          (bind _returnvalue_3 (Game|SpawnActorfromClass (Variables|Default|GetTurretPreviewClass) (Math|Transform|MakeTransform (LocalVariables|GetTurretPosistion) "0, 0, 0" "1.000000,1.000000,1.000000") "AlwaysSpawn" "MultiplyWithRoot" 0 0))
          (Variables|Default|SetTurretPreview _returnvalue_3)))
      (bind _returnvalue_4 (Class|KismetSystemLibrary|BoxTraceSingleforObjects (LocalVariables|GetTurretPosistion) (LocalVariables|GetTurretPosistion) "50.000000,50.000000,50.000000" "0, 0, 0" (Utilities|Array|MakeArray "ObjectTypeQuery8") false 0 "None" true "(R=1.000000,G=0.000000,B=0.000000,A=0.000000)" "(R=0.000000,G=1.000000,B=0.000000,A=0.000000)"))
      (bind _output_get_2 (Variables|Default|SetBuildIsValid (not _returnvalue_4)))
      (if _output_get_2
        (Rendering|Material|SetMaterial (Variables|/Game/TowerDefense/Blueprints/Towers/BP_BaseTowerPreview.BP_BaseTowerPreview_C|GetStaticMesh (Variables|Default|GetTurretPreview)) 0 "/Game/TowerDefense/Arte/Materiales/TorresConstruccion/Holograma.Holograma")
        (else
          (Rendering|Material|SetMaterial (Variables|/Game/TowerDefense/Blueprints/Towers/BP_BaseTowerPreview.BP_BaseTowerPreview_C|GetStaticMesh (Variables|Default|GetTurretPreview)) 0 "/Game/TowerDefense/Arte/Materiales/TorresConstruccion/Holograma_Inst_Red.Holograma_Inst_Red"))))))

(fn CleanBuildVariable
  (bind _turretpreview (Variables|Default|GetTurretPreview))
  (bind _frame (Variables|Default|GetFrame))
  (Variables|Default|SetTurretPreviewClass 0)
  (Variables|Default|SetTypeTurretClass 0)
  (if (Utilities|IsValid _turretpreview)
    (Actor|DestroyActor _turretpreview))
  (if (Utilities|IsValid _frame)
    (Actor|DestroyActor _frame))
  (Variables|Default|SetBuildIsValid false)
  (Variables|Default|SetBuildMode false)
  (Utilities|Time|ClearandInvalidateTimerbyHandle (Variables|Default|GetTimerTurretPosition)))

(fn PayTurret
  (params (A :type Float%20%28double-precision%29))
  (Variables|Default|SetPlayerMoney (- (Variables|Default|GetPlayerMoney) A))
  (Default|PhaseBuild (Variables|Default|GetMyHUD))
  (Default|CallWasteMoney))

(fn UpdateMoneyHUD
  (Default|SetMoneyText (Variables|Default|GetMyHUD) (Variables|Default|GetPlayerMoney)))

(fn SetTurretUpgrade
  (bind _myhud (Variables|Default|GetMyHUD))
  (bind _playercontroller (Variables|Default|GetPlayerController))
  (bind (_worldlocation _worlddirection) (Game|Player|ConvertMouseLocationToWorldSpace _playercontroller))
  (bind _cp_upgrademenu (Variables|/Game/TowerDefense/Blueprints/Widgets/WBP_HUD.WBP_HUD_C|GetCP_UpgradeMenu _myhud))
  (bind (_outhit _returnvalue) (Collision|LineTraceByChannel _worldlocation (+ _worldlocation (* _worlddirection 10000)) "TraceTypeQuery1" false 0 "None"))
  (if _returnvalue
    (bind _asbp_base_tower (Utilities|Casting|CastToBP_BaseTower (.HitActor (Collision|BreakHitResult _outhit)))
      (:then
        (Variables|Default|SetTurretUpgrade _asbp_base_tower)
        (Widget|SetVisibility _cp_upgrademenu "Visible"))
      (:CastFailed
        (Widget|SetVisibility _cp_upgrademenu "Hidden")
        (Variables|Default|SetTurretUpgrade 0)))))

(fn UpgradeDamage
  (Variables|Default|SetPlayerMoney (- (Variables|Default|GetPlayerMoney) (.CostDamageUpgrade (Utilities|GetClassDefaults (Utilities|GetClass (Variables|Default|GetTurretUpgrade))))))
  (Default|UpgradeDamage (Variables|Default|GetTurretUpgrade) 1.0)
  (Default|ActiveonOffUpgradeDamage (Variables|Default|GetMyHUD))
  (Default|CallWasteMoney))