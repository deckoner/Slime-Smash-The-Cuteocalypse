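; BP_SpawningEnemy is a tower defense enemy that splits into smaller spawns of BP_BaseEnemy when it dies.
; On death it always spawns three base enemies in a short line along world X, centered on its location, and passes them its GoalLocation.
; It then calls the parent death logic; the construction script only calls its parent.
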(event EventOnDeath
  (for _index (range -1 1)
    (Game|SpawnActorfromClass "/Game/TowerDefense/Blueprints/Enemies/BP_BaseEnemy.BP_BaseEnemy_C" (Math|Transform|MakeTransform (+ (* (* (Math|Vector|GetForwardVector "0, 0, 0") _index) 50) (Transformation|GetActorLocation)) "0, 0, 0" "1.000000,1.000000,1.000000") "AlwaysSpawn" "MultiplyWithRoot" 0 (Variables|Default|GetGoal%20Location) 0))
  (|CallParentFunction))

(fn ConstructionScript
  (|CallParentFunction))