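; BP_BaseEnemy is the base tower defense enemy that travels to a goal location and pays out money when killed.
; On possession it caches its AIC_Enemy controller, waits one tick, then hands it the goal location to move to.
; Incoming damage reduces health, and at zero the enemy destroys itself and awards money through GM_MyGameMode.
; DoDamage subtracts the enemy's damage from the player's HP through the same game mode.
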(event Game|Damage|EventAnyDamage
  (params (Damage :type Float%20%28single-precision%29) (DamageType :type Damage%20Type%20Object%20Reference) (InstigatedBy :type Controller%20Object%20Reference) (DamageCauser :type Actor%20Object%20Reference))
  ;[0.15 0.15 0.15 0.5] Take damage and gain money
  (Variables|Default|SetHealth%20Points (- (Variables|Default|GetHealth%20Points) Damage))
  (if (<= (Variables|Default|GetHealth%20Points) 0.0)
    (Actor|DestroyActor)
    (bind _asgm_my_game_mode (Utilities|Casting|CastToGM_MyGameMode (Game|GetGameMode)))
    (Default|GainMoney _asgm_my_game_mode (Variables|Default|GetMoney))))

(event EventPossessed
  (params (NewController :type Controller%20Object%20Reference))
  ;[0.15 0.15 0.15 0.5] Move to destination
  (bind _asaic_enemy (Utilities|Casting|CastToAIC_Enemy NewController))
  (Variables|Default|SetAIController _asaic_enemy)
  (Utilities|FlowControl|DelayUntilNextTick)
  (CallFunction|MovetoGoalLocation (Variables|Default|GetGoal%20Location)))

(fn ConstructionScript)

(fn MovetoGoalLocation
  (params (Goal%20Location :type Vector))
  (Default|MovetoGoalLocation (Variables|Default|GetAIController) Goal%20Location))

(fn DoDamage
  (bind _asgm_my_game_mode (Utilities|Casting|CastToGM_MyGameMode (Game|GetGameMode)))
  (Default|LoseHP _asgm_my_game_mode (Variables|Default|GetDamage)))