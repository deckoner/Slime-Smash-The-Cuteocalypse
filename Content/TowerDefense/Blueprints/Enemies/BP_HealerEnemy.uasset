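; Enemy Blueprint for a tower defense game that periodically heals other BP_BaseEnemy actors near it.
; Overlap events on its HealingRadius component keep an array of allies currently in range.
; A looping timer started on BeginPlay calls ReciveHealing on each tracked ally with HealingAmount and prints a debug message.
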(event OnComponentBeginOverlap(HealingRadius)
  (params (OverlappedComponent :type Primitive%20Component%20Object%20Reference) (OtherActor :type Actor%20Object%20Reference) (OtherComp :type Primitive%20Component%20Object%20Reference) (OtherBodyIndex :type Integer) (bFromSweep :type Boolean) (SweepResult :type Hit%20Result%20Structure%20%28by%20ref%29))
  (bind _asbp_base_enemy (Utilities|Casting|CastToBP_BaseEnemy OtherActor))
  (Utilities|Array|AddUnique (Variables|Default|GetAlliesArray) _asbp_base_enemy))

(event OnComponentEndOverlap(HealingRadius)
  (params (OverlappedComponent :type Primitive%20Component%20Object%20Reference) (OtherActor :type Actor%20Object%20Reference) (OtherComp :type Primitive%20Component%20Object%20Reference) (OtherBodyIndex :type Integer))
  (bind _asbp_base_enemy (Utilities|Casting|CastToBP_BaseEnemy OtherActor))
  (Utilities|Array|RemoveItem (Variables|Default|GetAlliesArray) _asbp_base_enemy))

(event Custom|Heall
  (Development|PrintText "Curo")
  (for _array_element (Variables|Default|GetAlliesArray)
    (Default|ReciveHealing _array_element (Variables|Default|GetHealingAmount))))

(event EventBeginPlay
  (Utilities|Time|SetTimerbyEvent (delegate Custom|Heall) 2.0 true))

(fn ConstructionScript
  (|CallParentFunction))