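; AIC_Enemy is the AI controller for tower defense enemies, moving each controlled pawn to a goal location.
; MoveToGoalLocation runs AI MoveTo; on success the BP_BaseEnemy pawn deals its damage and destroys itself, while failure prints a message.
; On possession it caches the pawn as BaseEnemyRef, though the move logic casts the controlled pawn again instead of using it.
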(event Custom|MoveToGoalLocation
  (params (Destination :type Vector))
  (bind _returnvalue (Pawn|GetControlledPawn))
  ;[0.15 0.15 0.15 0.5] Comment
  (bind _movementresult (AI|AIMoveTo _returnvalue Destination 0 5.0 false)
    (:OnSuccess
      (bind _asbp_base_enemy (Utilities|Casting|CastToBP_BaseEnemy _returnvalue))
      (Default|DoDamage _asbp_base_enemy)
      (Actor|DestroyActor _asbp_base_enemy))
    (:OnFail
      (Development|PrintString (Utilities|String|Append "Movement Failed: " (Utilities|String|EnumtoString _movementresult))))))

(event EventPossess
  (params (PossessedPawn :type Pawn%20Object%20Reference))
  ;[0.15 0.15 0.15 0.5] Comment
  (bind _asbp_base_enemy (Utilities|Casting|CastToBP_BaseEnemy PossessedPawn))
  (Variables|Default|SetBase%20Enemy%20Ref _asbp_base_enemy))

(fn ConstructionScript)