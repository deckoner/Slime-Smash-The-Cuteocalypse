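; AOE tower for the tower defense game that fires homing projectiles at all tracked enemies at once.
; Range overlap adds each BP_BaseEnemy to the Enemigos list, then starts or unpauses a one-second looping timer.
; Each tick spawns a projectile homing on every listed enemy's capsule.
; The empty-list check that clears the timer sits inside the loop, and this graph never removes enemies.
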(event OnComponentBeginOverlap(range)
  (params (OverlappedComponent :type Primitive%20Component%20Object%20Reference) (OtherActor :type Actor%20Object%20Reference) (OtherComp :type Primitive%20Component%20Object%20Reference) (OtherBodyIndex :type Integer) (bFromSweep :type Boolean) (SweepResult :type Hit%20Result%20Structure%20%28by%20ref%29))
  ;[0.15 0.15 0.15 0.5] Shoot on range enter
  (bind _asbp_base_enemy (Utilities|Casting|CastToBP_BaseEnemy OtherActor))
  (Utilities|Array|AddUnique (Variables|Default|GetEnemigos) _asbp_base_enemy)
  (if (> (Utilities|Array|Length (Variables|Default|GetEnemigos)) 0)
    (if (Utilities|Time|IsValidTimerHandle (Variables|Default|GetTimer))
      (Utilities|Time|UnpauseTimerbyHandle (Variables|Default|GetTimer))
      (else
        (bind _returnvalue (Utilities|Time|SetTimerbyEvent (delegate Custom|ShotProyectile) 1.0 true))
        (Variables|Default|SetTimer _returnvalue)))))

(event Custom|ShotProyectile
  ;[0.15 0.15 0.15 0.5] Shoot on range enter
  (for _array_element (Variables|Default|GetEnemigos)
    (CallFunction|SpawnHomingProjectile (Variables|/Script/Engine.Character|GetCapsuleComponent _array_element))
    (if (not (> (Utilities|Array|Length (Variables|Default|GetEnemigos)) 0))
      (Utilities|Time|ClearandInvalidateTimerbyHandle (Variables|Default|GetTimer)))))

(fn ConstructionScript
  (|CallParentFunction))