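; BP_DOTTower is a child tower Blueprint for the tower defense game, named as the DOT variant.
; On ShotProjectile it runs the parent's shot, then yaws its Cube mesh using a look-at rotation from the first entry in Enemigos to the Cube.
; An unwired failed test ("Prueba Fallida") would position, rotate, scale and show a component between shooter and enemy.
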(event EventShotProjectile
  (|CallParentFunction)
  (Transformation|SetWorldRotation (Variables|Default|GetCube) (Math|Rotator|MakeRotator 0.0 0.0 (.yaw (Math|Rotator|FindLookatRotation (Transformation|GetWorldLocation (Variables|/Script/Engine.Character|GetCapsuleComponent (Utilities|Array|Get(acopy) (Variables|Default|GetEnemigos)))) (Transformation|GetWorldLocation (Variables|Default|GetCube))))) false false))

(fn ConstructionScript
  (|CallParentFunction))