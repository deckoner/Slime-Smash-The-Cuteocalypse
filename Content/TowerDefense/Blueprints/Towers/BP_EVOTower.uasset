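; BP_EVOTower is a tower-defense tower that fires homing crystal projectiles at enemies entering its range sphere.
; Overlaps add enemies to an array and start or unpause a looping timer, which targets the first entry and spawns a projectile homing on its capsule.
; Tick turns the magic crystal toward the target.
; When the array is empty, the timer handler clears itself and slightly enlarges the range radius, updating overlaps.
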(event OnComponentBeginOverlap(range)
  (params (OverlappedComponent :type Primitive%20Component%20Object%20Reference) (OtherActor :type Actor%20Object%20Reference) (OtherComp :type Primitive%20Component%20Object%20Reference) (OtherBodyIndex :type Integer) (bFromSweep :type Boolean) (SweepResult :type Hit%20Result%20Structure%20%28by%20ref%29))
  ;[0.15 0.15 0.15 0.5] Shoot on range enter
  (bind _asbp_base_enemy (Utilities|Casting|CastToBP_BaseEnemy OtherActor))
  (Utilities|Array|AddUnique (Variables|Default|GetEnemigos) _asbp_base_enemy)
  (if (> (Utilities|Array|Length (Variables|Default|GetEnemigos)) 0)
    (if (Utilities|Time|IsValidTimerHandle (Variables|Default|GetTimer))
      (Utilities|Time|UnpauseTimerbyHandle (Variables|Default|GetTimer))
      (else
        (bind _returnvalue (Utilities|Time|SetTimerbyEvent (delegate Custom|CustomEvent_1) 0.5 true))
        (Variables|Default|SetTimer _returnvalue)))))

(event Custom|CustomEvent
  (params (Homing%20Target%20Component :type Scene%20Component%20Object%20Reference))
  ;[0.15 0.15 0.15 0.5] Projectile spawn
  (bind _returnvalue (Game|SpawnActorfromClass "/Game/TowerDefense/Blueprints/Towers/BP_Projectile_Crystal.BP_Projectile_Crystal_C" (Transformation|GetWorldTransform (Variables|Default|GetShootPoint)) "AdjustIfPossibleButAlwaysSpawn" "MultiplyWithRoot" 0 (Variables|Default|GetDamage) 0))
  (Variables|/Script/Engine.ProjectileMovementComponent|SetHomingTargetComponent (Variables|/Game/TowerDefense/Blueprints/Towers/BP_Projectile.BP_Projectile_C|GetProjectileMovement _returnvalue) Homing%20Target%20Component))

(event Custom|CustomEvent_1
  ;[0.15 0.15 0.15 0.5] Shoot on range enter
  (bind _output_get (Variables|Default|SetTarget (Utilities|Array|Get(acopy) (Variables|Default|GetEnemigos))))
  (CallFunction|SpawnHomingProjectile (Variables|/Script/Engine.Character|GetCapsuleComponent _output_get))
  (if (not (> (Utilities|Array|Length (Variables|Default|GetEnemigos)) 0))
    (Utilities|Time|ClearandInvalidateTimerbyHandle (Variables|Default|GetTimer))
    (Components|Sphere|SetSphereRadius (Variables|Default|Getrange) (+ (Variables|/Script/Engine.SphereComponent|GetSphereRadius (Variables|Default|Getrange)) 1.0) true)))

(event EventTick
  (params (DeltaSeconds :type Float%20%28single-precision%29))
  (Transformation|SetRelativeRotation (Variables|Default|GetMagic%20Crystal) (Math|Rotator|FindLookatRotation (Transformation|GetWorldLocation (Variables|Default|GetMagic%20Crystal)) (Transformation|GetActorLocation (Variables|Default|GetTarget))) false false))

(fn ConstructionScript
  (|CallParentFunction))