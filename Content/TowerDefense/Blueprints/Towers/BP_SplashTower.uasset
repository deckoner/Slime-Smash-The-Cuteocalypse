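; BP_SplashTower is a tower defense tower that fires homing projectiles at enemies within its Range component.
; Overlap events maintain the Enemigos list of BP_BaseEnemy actors and start a looping one-second timer, cleared when the list empties.
; Each tick of that timer spawns a BP_Projectile at ShootPoint, passing Damage and homing on the first listed enemy's capsule.
; No splash logic appears in this Blueprint itself.
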(event OnComponentEndOverlap(range)
  (params (OverlappedComponent :type Primitive%20Component%20Object%20Reference) (OtherActor :type Actor%20Object%20Reference) (OtherComp :type Primitive%20Component%20Object%20Reference) (OtherBodyIndex :type Integer))
  (bind _enemigos (Variables|Default|GetEnemigos))
  ;[0.15 0.15 0.15 0.5] Stop shootiong on range exit
  (bind _asbp_base_enemy (Utilities|Casting|CastToBP_BaseEnemy OtherActor))
  (Utilities|Array|RemoveItem _enemigos _asbp_base_enemy)
  (if (not (> (Utilities|Array|Length _enemigos) 0))
    (Utilities|Time|ClearandInvalidateTimerbyHandle (Variables|Default|GetTimer))))

(event OnComponentBeginOverlap(range)
  (params (OverlappedComponent :type Primitive%20Component%20Object%20Reference) (OtherActor :type Actor%20Object%20Reference) (OtherComp :type Primitive%20Component%20Object%20Reference) (OtherBodyIndex :type Integer) (bFromSweep :type Boolean) (SweepResult :type Hit%20Result%20Structure%20%28by%20ref%29))
  ;[0.15 0.15 0.15 0.5] Shoot on range enter
  (bind _asbp_base_enemy (Utilities|Casting|CastToBP_BaseEnemy OtherActor))
  (Utilities|Array|AddUnique (Variables|Default|GetEnemigos) _asbp_base_enemy)
  (if (> (Utilities|Array|Length (Variables|Default|GetEnemigos)) 0)
    (if (Utilities|Time|IsValidTimerHandle (Variables|Default|GetTimer))
      (Utilities|Time|UnpauseTimerbyHandle (Variables|Default|GetTimer))
      (else
        (bind _returnvalue (Utilities|Time|SetTimerbyEvent (delegate Custom|ShotProjectile) 1.0 true))
        (Variables|Default|SetTimer _returnvalue)))))

(event Custom|SpawnHomingProjectile
  (params (Homing%20Target%20Component :type Scene%20Component%20Object%20Reference))
  ;[0.15 0.15 0.15 0.5] Projectile spawn
  (bind _returnvalue (Game|SpawnActorfromClass "/Game/TowerDefense/Blueprints/Towers/BP_Projectile.BP_Projectile_C" (Transformation|GetWorldTransform (Variables|Default|GetShootPoint)) "AdjustIfPossibleButAlwaysSpawn" "MultiplyWithRoot" 0 (Variables|Default|GetDamage) 0))
  (Variables|/Script/Engine.ProjectileMovementComponent|SetHomingTargetComponent (Variables|/Game/TowerDefense/Blueprints/Towers/BP_Projectile.BP_Projectile_C|GetProjectileMovement _returnvalue) Homing%20Target%20Component))

(event Custom|ShotProjectile
  ;[0.15 0.15 0.15 0.5] Shoot on range enter
  (CallFunction|SpawnHomingProjectile (Variables|/Script/Engine.Character|GetCapsuleComponent (Utilities|Array|Get(acopy) (Variables|Default|GetEnemigos))))
  (if (not (> (Utilities|Array|Length (Variables|Default|GetEnemigos)) 0))
    (Utilities|Time|ClearandInvalidateTimerbyHandle (Variables|Default|GetTimer))))

(fn ConstructionScript)