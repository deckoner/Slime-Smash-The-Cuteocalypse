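; Tower defense spawner actor that releases configured waves of enemies at its location and gives each one the Destination's location as its goal.
; WaveArray holds waves made of enemy groups, each defining type, count, spawn interval and start delay.
; A looping timer spawns each group, then chains to the next.
; After a wave's last group, the wave index advances and spawning pauses until EnemySpawnCaller runs again.
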(event Custom|SpawnEnemy
  (if (>= (Variables|Default|GetSpawnedEnemies) (CallFunction|GetNumEnemies))
    (Utilities|Time|ClearandInvalidateTimerbyHandle (Variables|Default|GetTimer))
    (Math|Integer|IncrementInt (Variables|Default|GetEnemyWaveArray)
      (:%20%20
        (Variables|Default|SetSpawnedEnemies 0)
        (CallFunction|SpawnArray)))
    (else
      (CallFunction|SpawnActorEnemy))))

(event Custom|SpawnArray
  (Variables|Default|SetWave (.wave (Utilities|Array|Get(acopy) (Variables|Default|GetWaveArray) (Variables|Default|GetWaveCouter))))
  (if (>= (Variables|Default|GetEnemyWaveArray) (Utilities|Array|Length (Variables|Default|GetWave)))
    (Variables|Default|SetSpawnedEnemies 0)
    (Variables|Default|SetEnemyWaveArray 0)
    (Math|Integer|IncrementInt (Variables|Default|GetWaveCouter))
    (else
      (bind _returnvalue (Utilities|Time|SetTimerbyEvent (delegate Custom|SpawnEnemy) (CallFunction|GetSpawnTimer) true false (CallFunction|GetWaveTimer)))
      (Variables|Default|SetTimer _returnvalue))))

(event EventBeginPlay
  (bind _asgm_my_game_mode (Utilities|Casting|CastToGM_MyGameMode (Game|GetGameMode)))
  (Variables|Default|SetAs%20GM%20My%20Game%20Mode _asgm_my_game_mode))

(fn ConstructionScript)

(fn GetNumEnemies
  (return (.numenemies (Utilities|Array|Get(acopy) (Variables|Default|GetWave) (Variables|Default|GetEnemyWaveArray)))))

(fn GetEnemyType
  (return (.enemytype (Utilities|Array|Get(acopy) (Variables|Default|GetWave) (Variables|Default|GetEnemyWaveArray)))))

(fn GetSpawnTimer
  (return (.spawntimer (Utilities|Array|Get(acopy) (Variables|Default|GetWave) (Variables|Default|GetEnemyWaveArray)))))

(fn GetWaveTimer
  (return (.wavetimer (Utilities|Array|Get(acopy) (Variables|Default|GetWave) (Variables|Default|GetEnemyWaveArray)))))

(fn SpawnActorEnemy
  (bind _returnvalue (Game|SpawnActorfromClass (CallFunction|GetEnemyType) (Math|Transform|MakeTransform (Transformation|GetActorLocation) "0, 0, 0" "1.000000,1.000000,1.000000") "AdjustIfPossibleButAlwaysSpawn" "MultiplyWithRoot" 0 0))
  (Math|Integer|IncrementInt (Variables|Default|GetSpawnedEnemies)
    (:%20%20
      (Variables|/Game/TowerDefense/Blueprints/Enemies/BP_BaseEnemy.BP_BaseEnemy_C|SetGoal%20Location _returnvalue (Transformation|GetWorldLocation (Variables|Default|GetDestination))))))

(fn EnemySpawnCaller
  (CallFunction|SpawnArray))