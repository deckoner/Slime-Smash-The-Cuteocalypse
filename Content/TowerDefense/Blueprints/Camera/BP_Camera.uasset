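; BP_Camera is the fixed overhead camera for a tower defense game and doubles as the player's input handler.
; Its construction script pins it to a hard-coded, downward-angled transform, and BeginPlay caches GM_MyGameMode and shows the mouse cursor.
; Left click, right click and Space forward to the game mode to build a turret, clear build state and start a round.
; An UpdateTurretPosition call is left unconnected.
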(event EventBeginPlay
  ;[0.15 0.15 0.15 0.5] Empezar juego
  (bind _asgm_my_game_mode (Utilities|Casting|CastToGM_MyGameMode (Game|GetGameMode)))
  (Variables|Default|SetAs%20GM%20My%20Game%20Mode _asgm_my_game_mode)
  (Variables|/Script/Engine.PlayerController|SetbShowMouseCursor (Game|GetPlayerController 0) true))

(event Input|KeyboardEvents|SpaceBar
  (params (Key :type Key%20Structure :default "None"))
  ;[0.15 0.15 0.15 0.5] Empezar Oleada
  (:Pressed
    (Default|StartRound (Variables|Default|GetAs%20GM%20My%20Game%20Mode))))

(event Input|MouseEvents|LeftMouseButton
  (params (Key :type Key%20Structure :default "None"))
  ;[0.15 0.15 0.15 0.5] CiIck Create Turret
  (:Pressed
    (Default|BuildTurret (Variables|Default|GetAs%20GM%20My%20Game%20Mode))))

(event Input|MouseEvents|RightMouseButton
  (params (Key :type Key%20Structure :default "None"))
  ;[0.15 0.15 0.15 0.5] Click Cancel Turret
  (:Pressed
    (Default|CleanBuildVariable (Variables|Default|GetAs%20GM%20My%20Game%20Mode))))

(fn ConstructionScript
  (Transformation|SetActorLocationAndRotation "-2200.000000,-70.000000,2750.000000" "-60.000000,0.000000,0.000000"))