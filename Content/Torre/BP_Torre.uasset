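; BP_Torre is a tower that automatically fires projectiles at BP_Base_Enemigo actors inside its RangoTorre overlap volume.
; Entering enemies join ListaObjetivos and start a looping Cadencia timer, which is cleared once the list empties.
; Each tick of that timer calls Disparar, spawning a Proyectil at the Billboard with the first listed enemy's capsule and Dano.
; Disparar also prints that target's location for debugging.
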(event OnComponentBeginOverlap(RangoTorre)
  (params (OverlappedComponent :type Primitive%20Component%20Object%20Reference) (OtherActor :type Actor%20Object%20Reference) (OtherComp :type Primitive%20Component%20Object%20Reference) (OtherBodyIndex :type Integer) (bFromSweep :type Boolean) (SweepResult :type Hit%20Result%20Structure%20%28by%20ref%29))
  ;[0.15 0.15 0.15 0.5] Funcion de disparo al entrar
  (bind _asbp_base_enemigo (Utilities|Casting|CastToBP_Base_Enemigo OtherActor))
  (Utilities|Array|Add (Variables|Default|GetListaObjetivos) _asbp_base_enemigo)
  (if (not (Variables|Default|GetDisparando))
    (Variables|Default|SetDisparando true)
    (bind _returnvalue (Utilities|Time|SetTimerbyEvent (delegate Custom|Iniciar%20disparos) (Variables|Default|GetCadencia) true))
    (Variables|Default|SetTimerEvent _returnvalue)))

(event OnComponentEndOverlap(RangoTorre)
  (params (OverlappedComponent :type Primitive%20Component%20Object%20Reference) (OtherActor :type Actor%20Object%20Reference) (OtherComp :type Primitive%20Component%20Object%20Reference) (OtherBodyIndex :type Integer))
  (bind _listaobjetivos (Variables|Default|GetListaObjetivos))
  ;[0.15 0.15 0.15 0.5] Eliminar Enemigo de la Array al salir
  (bind _asbp_base_enemigo (Utilities|Casting|CastToBP_Base_Enemigo OtherActor))
  (Utilities|Array|RemoveItem _listaobjetivos _asbp_base_enemigo)
  (if (Utilities|Array|IsEmpty _listaobjetivos)
    (Utilities|Time|ClearandInvalidateTimerbyHandle (Variables|Default|GetTimerEvent))
    (Variables|Default|SetDisparando false)))

(event Custom|Iniciar%20disparos
  ;[0.15 0.15 0.15 0.5] Funcion de disparo al entrar
  (CallFunction|Disparar))

(fn ConstructionScript)

(fn Disparar
  (bind _listaobjetivos (Variables|Default|GetListaObjetivos))
  (bind _output (Utilities|Array|Get(acopy) _listaobjetivos))
  (bind _capsulecomponent (Variables|/Script/Engine.Character|GetCapsuleComponent _output))
  (Game|SpawnActorfromClass (Variables|Default|GetProyectil) (Transformation|GetWorldTransform (Variables|Default|GetBillboard)) "Undefined" "MultiplyWithRoot" 0 _capsulecomponent (Variables|Default|GetDano) 0)
  (Development|PrintString (Utilities|String|ToString(Vector) (Transformation|GetWorldLocation _capsulecomponent)) true true "(R=0.160884,G=1.000000,B=0.000000,A=1.000000)" 5.0))