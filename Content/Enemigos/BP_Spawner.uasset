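; BP_Spawner is the tower defense enemy spawner, registering itself with GM_TowerDefenser and spawning timed waves of enemies at its own location.
; EstablecerWave loads the current round's wave list, and EmpezarOleada starts running it.
; A looping timer spawns each wave's enemy type, passing the Billboard position as destination, until its count is reached.
; FinalOleada then advances to the next wave, notifying the game mode when the list is exhausted.
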(event Custom|CustomEvent
  (bind _enemywave (Variables|Default|GetEnemyWave))
  (bind _oleadaactual (Variables|Default|GetOleadaActual))
  (bind _output (Utilities|Array|Get(acopy) _enemywave _oleadaactual))
  ;[0.15 0.15 0.15 0.5] Oleada
  (if (>= (Variables|Default|GetNEnemigo) (.numenemigos _output))
    (CallFunction|FinalOleada)
    (else
      (CallFunction|SpanwEnemigo (.tipoenemigo _output)))))

(event Custom|Oleada
  (bind _enemywave (Variables|Default|GetEnemyWave))
  (bind _oleadaactual (Variables|Default|GetOleadaActual))
  (bind _output (Utilities|Array|Get(acopy) _enemywave _oleadaactual))
  ;[0.15 0.15 0.15 0.5] Oleada
  (if (>= _oleadaactual (Utilities|Array|Length _enemywave))
    (Default|TerminarOleadas (Variables|Default|GetAs%20GM%20Tower%20Defenser))
    (else
      (bind _returnvalue (Utilities|Time|SetTimerbyEvent (delegate Custom|CustomEvent) (.timeroleada _output) true false (.timerronda _output)))
      (Variables|Default|SetTimerEvent _returnvalue))))

(event EventBeginPlay
  ;[0.15 0.15 0.15 0.5] Inicio
  (Utilities|FlowControl|DelayUntilNextTick)
  (Variables|Default|SetDestinoEnemigo (Transformation|GetWorldLocation (Variables|Default|GetBillboard)))
  (CallFunction|EstablecerWave)
  (bind _asgm_tower_defenser (Utilities|Casting|CastToGM_TowerDefenser (Game|GetGameMode)))
  (Variables|/Game/GM_TowerDefenser.GM_TowerDefenser_C|SetSpawner _asgm_tower_defenser self)
  (bind _asgm_tower_defenser_2 (Utilities|Casting|CastToGM_TowerDefenser (Game|GetGameMode)))
  (Variables|Default|SetAs%20GM%20Tower%20Defenser _asgm_tower_defenser_2))

(fn ConstructionScript)

(fn FinalOleada
  (Math|Integer|IncrementInt (Variables|Default|GetOleadaActual)
    (:%20%20
      (Variables|Default|SetNEnemigo 0)
      (Utilities|Time|ClearandInvalidateTimerbyHandle (Variables|Default|GetTimerEvent))
      (CallFunction|Oleada))))

(fn SpanwEnemigo
  (params (Class :type BP%20Base%20Enemigo%20Class%20Reference))
  (bind _returnvalue (Game|SpawnActorfromClass Class (Math|Transform|MakeTransform (Transformation|GetActorLocation) "0, 0, 0" "1.000000,1.000000,1.000000") "AdjustIfPossibleButAlwaysSpawn" "MultiplyWithRoot" 0 0))
  (Variables|/Game/Enemigos/BP_Base_Enemigo.BP_Base_Enemigo_C|SetDestino _returnvalue (Variables|Default|GetDestinoEnemigo))
  (Math|Integer|IncrementInt (Variables|Default|GetNEnemigo)))

(fn EmpezarOleada
  (if (not (>= (Variables|Default|GetnOleada) (Utilities|Array|Length (Variables|Default|GetOleadas))))
    (Variables|Default|SetTotalOleadas 0)
    (Variables|Default|SetOleadaActual 0)
    (CallFunction|Oleada)
    (Math|Integer|IncrementInt (Variables|Default|GetnOleada))))

(fn EstablecerWave
  (Variables|Default|SetEnemyWave (.oleadas (Utilities|Array|Get(acopy) (Variables|Default|GetOleadas) (Variables|Default|GetnOleada)))))