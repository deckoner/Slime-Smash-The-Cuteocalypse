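; BP_Base_Enemigo is the base enemy for a tower defense game.
; When possessed, it stores its AIC_enemy controller and, a tick later, orders it to move to its destination.
; RecibirDano subtracts health and, at zero or below, awards Parne to GM_TowerDefenser before destroying the enemy.
; HacerDano passes the enemy's damage to the game mode and destroys it.
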(event EventPossessed
  (params (NewController :type Controller%20Object%20Reference))
  ;[0.15 0.15 0.15 0.5] Ir hacia el objetivo
  (bind _asaic_enemy (Utilities|Casting|CastToAIC_enemy NewController))
  (Variables|Default|SetAICEnemy _asaic_enemy)
  (Utilities|FlowControl|DelayUntilNextTick)
  (Default|IrObjetivo (Variables|Default|GetAICEnemy) (Variables|Default|GetDestino)))

(event EventBeginPlay
  ;[0.15 0.15 0.15 0.5] Optener el GM
  (bind _asgm_tower_defenser (Utilities|Casting|CastToGM_TowerDefenser (Game|GetGameMode)))
  (Variables|Default|SetAs%20GM%20Tower%20Defenser _asgm_tower_defenser))

(fn ConstructionScript)

(fn RecibirDano
  (params (DanoRecibido :type Integer))
  (bind _output_get (Variables|Default|SetVida (- (Variables|Default|GetVida) DanoRecibido)))
  (if (<= _output_get 0)
    (Default|AnadirParne (Variables|Default|GetAs%20GM%20Tower%20Defenser) (Variables|Default|GetParneDado))
    (Actor|DestroyActor)))

(fn HacerDano
  (Default|HacerDano (Variables|Default|GetAs%20GM%20Tower%20Defenser) (Variables|Default|GetDano))
  (Actor|DestroyActor))